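; Skeleton enemy character that carries a spawned sword, senses and fights the player, and supports being lock-on targeted.
; BeginPlay attaches the sword, passes it to a trace component and starts Skeleton_BT, which receives state through a Behaviour blackboard enum.
; Pawn sensing, sphere exit and damage switch that state, with a retriggerable delay for hit recovery.
; Attacks play random montages; death stops AI logic and releases the player's lock-on.
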(event OnSeePawn(PawnSensing)
  (params (Pawn :type Pawn%20Object%20Reference))
  ;[1 1 1] Handle enemy vision
  (if (and (== Pawn (Game|GetPlayerCharacter 0)) (Utilities|Enum|NotEqual(Enum) (Variables|Default|Getbehaviour) "NewEnumerator0"))
    (Variables|Default|Setbehaviour "NewEnumerator3")
    (AI|Components|Blackboard|SetValueasEnum (AI|GetBlackboard 0) (Utilities|Name|MakeLiteralName "eBehaviour") (Variables|Default|Getbehaviour))))

(event OnComponentEndOverlap(Sphere)
  (params (OverlappedComponent :type Primitive%20Component%20Object%20Reference) (OtherActor :type Actor%20Object%20Reference) (OtherComp :type Primitive%20Component%20Object%20Reference) (OtherBodyIndex :type Integer))
  ;[1 1 1] Escape enemy
  (Utilities|Casting|CastToBP_ThirdPersonCharacter OtherActor)
  (Variables|Default|Setbehaviour "NewEnumerator1")
  (AI|Components|Blackboard|SetValueasEnum (AI|GetBlackboard 0) (Utilities|Name|MakeLiteralName "eBehaviour") (Variables|Default|Getbehaviour)))

(event Custom|Attack
  ;[1 1 1] Attack System
  (bind _returnvalue (Animation|PlayAnimMontage (.OutItem (Utilities|Array|Random (Variables|Default|GetAttackAnimations))) 1.0 "None"))
  (Variables|Default|Setattacklength _returnvalue))

(event EventBeginPlay
  ;[1 1 1] Set up enemy character
  (bind _returnvalue (Game|SpawnActorfromClass (Variables|Default|Getsword) (Transformation|GetSocketTransform (Variables|Character|GetMesh) "sword" "RTS_World") "Undefined" 0 0))
  (bind _asbp_basesword (Utilities|Casting|CastToBP_Basesword _returnvalue))
  (bind _output_get (Variables|Default|Setswordref _asbp_basesword))
  (Transformation|AttachComponentToComponent _output_get (Variables|Character|GetMesh) "sword" "SnapToTarget" "SnapToTarget" "SnapToTarget" true)
  (Variables|/Game/Equipment/TraceComponent.TraceComponent_C|Setswordref (Variables|Default|GetTraceComponent) (Variables|Default|Getswordref))
  (AI|RunBehaviorTree (AI|GetAIController self) "/Game/Enemy/BehaviourTree/Skeleton_BT.Skeleton_BT")
  (bind _asbp_third_person_character (Utilities|Casting|CastToBP_ThirdPersonCharacter (Game|GetPlayerCharacter 0)))
  (Variables|Default|SetPlayerRef _asbp_third_person_character)
  (Rendering|SetVisibility (Variables|Default|GetLockOn) false false)
  (AI|Components|Blackboard|SetValueasEnum (AI|GetBlackboard 0) (Utilities|Name|MakeLiteralName "eBehaviour") (Variables|Default|Getbehaviour))
  (Variables|/Game/Equipment/RotatingComponent.RotatingComponent_C|SetTarget (Variables|Default|GetRotatingComponent) (Game|GetPlayerCharacter 0)))

(event Collision|EventActorBeginOverlap
  (params (OtherActor :type Actor%20Object%20Reference)))

(event EventTick
  (params (DeltaSeconds :type Float%20%28single-precision%29)))

(event Game|Damage|EventAnyDamage
  (params (Damage :type Float%20%28single-precision%29) (DamageType :type Damage%20Type%20Object%20Reference) (InstigatedBy :type Controller%20Object%20Reference) (DamageCauser :type Actor%20Object%20Reference))
  (bind _playerref (Variables|Default|GetPlayerRef))
  (bind _target_actor (Variables|/Game/ThirdPerson/Blueprints/BP_ThirdPersonCharacter.BP_ThirdPersonCharacter_C|GetTarget%20Actor _playerref))
  ;[1 1 1] Damage system
  (Variables|Default|Setbehaviour "NewEnumerator0")
  (AI|Components|Blackboard|SetValueasEnum (AI|GetBlackboard 0) (Utilities|Name|MakeLiteralName "eBehaviour") (Variables|Default|Getbehaviour))
  (bind _output_get (Variables|Default|SetHealth (- (Variables|Default|GetHealth) Damage)))
  (if (<= _output_get 0.0)
    (Utilities|FlowControl|DoOnce false
      (:Completed
        (AI|Logic|StopLogic (Variables|/Script/AIModule.AIController|GetBrainComponent (AI|GetAIController self)) "die")
        (Variables|Default|SetEnemyDead? true)
        (Animation|PlayAnimMontage "/Game/Enemy/Animation/SkeleDeath_Montage.SkeleDeath_Montage" 1.0 "None")
        (Utilities|IsValid _target_actor
          (:Is%20Valid
            (if (== _target_actor self)
              (Default|DisengageLockON (Variables|Default|GetPlayerRef)))))))
    (else
      (Animation|PlayAnimMontage "/Game/Enemy/Animation/Skele_Hit_Montage.Skele_Hit_Montage" 1.0 "None")
      (Utilities|FlowControl|RetriggerableDelay (Variables|Default|GetDamagetime))
      (Variables|Default|Setbehaviour "NewEnumerator3")
      (AI|Components|Blackboard|SetValueasEnum (AI|GetBlackboard 0) (Utilities|Name|MakeLiteralName "eBehaviour") (Variables|Default|Getbehaviour)))))

(event EventOnSelected
  ;[1 1 1] Handle Lock on
  (Rendering|SetVisibility (Variables|Default|GetLockOn) true false))

(event EventOnDeSeleccted
  ;[1 1 1] Handle Lock on
  (Rendering|SetVisibility (Variables|Default|GetLockOn) false false))

(fn ConstructionScript)

(fn IsDead
  (return (Variables|Default|GetEnemyDead?)))